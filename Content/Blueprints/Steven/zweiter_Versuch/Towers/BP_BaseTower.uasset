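; Base tower Blueprint for a tower defense setup, tracking BP_Enemy actors that enter or leave its Range component in EnemiesInRange.
; Tick counts down an attack cooldown and calls Attack once it expires, resetting it only on success, so failed attacks retry every frame.
; Attack is a stub returning false, apparently for child towers to override.
; Getters expose the possible upgrades and the tower's placing block.
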(event OnComponentBeginOverlap(Range)
  (params (OverlappedComponent :type Primitive%20Component%20Object%20Reference) (OtherActor :type Actor%20Object%20Reference) (OtherComp :type Primitive%20Component%20Object%20Reference) (OtherBodyIndex :type Integer) (bFromSweep :type Boolean) (SweepResult :type Hit%20Result%20Structure%20%28by%20ref%29))
  (bind _asbp_enemy (Utilities|Casting|CastToBP_Enemy OtherActor))
  (Utilities|Array|AddUnique (Variables|Default|GetEnemiesInRange) _asbp_enemy))

(event OnComponentEndOverlap(Range)
  (params (OverlappedComponent :type Primitive%20Component%20Object%20Reference) (OtherActor :type Actor%20Object%20Reference) (OtherComp :type Primitive%20Component%20Object%20Reference) (OtherBodyIndex :type Integer))
  (bind _asbp_enemy (Utilities|Casting|CastToBP_Enemy OtherActor))
  (Utilities|Array|RemoveItem (Variables|Default|GetEnemiesInRange) _asbp_enemy))

(event EventBeginPlay)

(event Collision|EventActorBeginOverlap
  (params (OtherActor :type Actor%20Object%20Reference)))

(event EventTick
  (params (DeltaSeconds :type Float%20%28single-precision%29))
  (bind _output_get (Variables|Default|SetAttackCdTimer (- (Variables|Default|GetAttackCdTimer) DeltaSeconds)))
  (if (<= _output_get 0.0)
    (bind _success (CallFunction|Attack))
    (if _success
      (Variables|Default|SetAttackCdTimer (Variables|Default|GetAttackCd)))))

(fn ConstructionScript)

(fn GetPossibleUpgrades
  (return (Variables|Default|GetPossibleUpgrades)))

(fn GetTowerPlacingBlock
  (return (Variables|Default|GetTowerPlacingBlock)))

(fn Attack
  (return false))