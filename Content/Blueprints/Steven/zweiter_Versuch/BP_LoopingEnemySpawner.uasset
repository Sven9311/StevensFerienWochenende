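; BP_LoopingEnemySpawner is a child enemy spawner that restarts its wave sequence instead of ending it.
; Each Tick runs the parent's logic, then checks whether the current wave index is strictly greater than the wave array's length.
; When it is, it resets the index, spawn-finished flag and spawned-enemy count, and reloads the timer from the first wave.
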(event EventBeginPlay
  (|CallParentFunction) ; This node is disabled and will not be called.\nDrag off pins to build functionality.
)

(event Collision|EventActorBeginOverlap
  (params (OtherActor :type Actor%20Object%20Reference))
  (|CallParentFunction OtherActor) ; This node is disabled and will not be called.\nDrag off pins to build functionality.
)

(event EventTick
  (params (DeltaSeconds :type Float%20%28single-precision%29))
  (|CallParentFunction DeltaSeconds)
  (if (CallFunction|CurrentWaveIsBiggerThanMax)
    (Variables|Default|SetCurrentWave 0)
    (Variables|Default|SetTimer (.wavetimer (Utilities|Array|Get(acopy) (Variables|Default|GetWave))))
    (Variables|Default|SetWaveSpawnFinished false)
    (Variables|Default|SetNumOfSpawnedEnemies 0)))

(fn ConstructionScript
  (|CallParentFunction))

(fn CurrentWaveIsBiggerThanMax
  (return (> (Variables|Default|GetCurrentWave) (Utilities|Array|Length (Variables|Default|GetWave)))))