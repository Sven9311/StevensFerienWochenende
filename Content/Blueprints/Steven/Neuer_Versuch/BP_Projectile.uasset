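; Homing tower projectile that destroys the enemy it hits.
; InitializeHoming stores the target and, if it is valid, points ProjectileMovement's homing at that target's root component.
; On a sphere hit with a BP_BaseEnemy2, it tells OwnerTower to stop tracking that enemy, then destroys itself and the enemy, with no damage step.
; Leftover debug prints and earlier removal and homing logic remain unconnected in the event graph.
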(event OnComponentHit(SphereCollision)
  (params (HitComponent :type Primitive%20Component%20Object%20Reference) (OtherActor :type Actor%20Object%20Reference) (OtherComp :type Primitive%20Component%20Object%20Reference) (NormalImpulse :type Vector :default "0, 0, 0") (Hit :type Hit%20Result%20Structure%20%28by%20ref%29))
  (bind _asbp_base_enemy_2 (Utilities|Casting|CastToBP_BaseEnemy2 OtherActor))
  (Default|RemoveEnemyfromTracking (Variables|Default|GetownerTower) _asbp_base_enemy_2)
  (Actor|DestroyActor)
  (Actor|DestroyActor OtherActor))

(event EventBeginPlay)

(event Collision|EventActorBeginOverlap
  (params (OtherActor :type Actor%20Object%20Reference)))

(event EventTick
  (params (DeltaSeconds :type Float%20%28single-precision%29)))

(fn ConstructionScript)

(fn InitializeHoming
  (params (Target :type Actor%20Object%20Reference))
  (Variables|Default|SetTargetEnemy Target)
  (if (Utilities|IsValid (Variables|Default|GetTargetEnemy))
    (Variables|/Script/Engine.ProjectileMovementComponent|SetHomingTargetComponent (Variables|Default|GetProjectileMovement) (Variables|/Script/Engine.Actor|GetRootComponent (Variables|Default|GetTargetEnemy)))))