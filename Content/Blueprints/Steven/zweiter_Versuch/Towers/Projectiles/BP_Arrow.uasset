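; BP_Arrow is a tower projectile that homes in on an assigned enemy target.
; Each tick it re-aims at the target and moves by Speed without sweeping.
; If the target is lost, it keeps flying along its last direction and self-destructs after two seconds, or at once if it has no direction.
; Its capsule overlap applies the assigned Damage to any BP_Enemy it touches, then destroys the arrow.
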(event OnComponentBeginOverlap(Cone)
  (params (OverlappedComponent :type Primitive%20Component%20Object%20Reference) (OtherActor :type Actor%20Object%20Reference) (OtherComp :type Primitive%20Component%20Object%20Reference) (OtherBodyIndex :type Integer) (bFromSweep :type Boolean) (SweepResult :type Hit%20Result%20Structure%20%28by%20ref%29)))

(event OnComponentBeginOverlap(Capsule)
  (params (OverlappedComponent :type Primitive%20Component%20Object%20Reference) (OtherActor :type Actor%20Object%20Reference) (OtherComp :type Primitive%20Component%20Object%20Reference) (OtherBodyIndex :type Integer) (bFromSweep :type Boolean) (SweepResult :type Hit%20Result%20Structure%20%28by%20ref%29))
  (bind _asbp_enemy (Utilities|Casting|CastToBP_Enemy OtherActor))
  (Game|Damage|ApplyDamage _asbp_enemy (Variables|Default|GetDamage) 0 0)
  (Actor|DestroyActor))

(event Custom|DestroyArrow
  (Actor|DestroyActor))

(event EventBeginPlay)

(event Collision|EventActorBeginOverlap
  (params (OtherActor :type Actor%20Object%20Reference)))

(event EventTick
  (params (DeltaSeconds :type Float%20%28single-precision%29))
  (if (Utilities|IsValid (Variables|Default|GetTarget))
    (Variables|Default|SetDirection (Math|Vector|Normalize (- (Transformation|GetActorLocation (Variables|Default|GetTarget)) (Transformation|GetActorLocation))))
    (CallFunction|Move DeltaSeconds)
    (elif (CallFunction|IsMoving)
      (CallFunction|Move DeltaSeconds)
      (if (not (Class|KismetSystemLibrary|TimerExistsHandle (Variables|Default|GetDestroyTimerHandle)))
        (bind _returnvalue (Utilities|Time|SetTimerbyEvent (delegate Custom|DestroyArrow) 2.0))
        (Variables|Default|SetDestroyTimerHandle _returnvalue))
      (else
        (Actor|DestroyActor)))))

(fn ConstructionScript)

(fn SetTarget
  (params (EnemyTarget :type BP%20Enemy%20Object%20Reference))
  (Variables|Default|SetTarget EnemyTarget))

(fn SetDamage
  (params (NewDamage :type Float%20%28double-precision%29))
  (Variables|Default|SetDamage NewDamage))

(fn IsMoving
  (return (not (Math|Vector|VectorIsNearlyZero (Variables|Default|GetDirection)))))

(fn Move
  (params (DeltaTime :type Float%20%28double-precision%29))
  (Transformation|SetActorLocation (+ (* DeltaTime (Variables|Default|GetDirection) (Variables|Default|GetSpeed)) (Transformation|GetActorLocation)) false false))