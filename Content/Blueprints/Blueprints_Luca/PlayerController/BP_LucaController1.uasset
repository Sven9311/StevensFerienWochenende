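; Player controller that provides right-click-to-move control with a visible mouse cursor.
; On BeginPlay it adds the IMC_Sven Enhanced Input mapping context, caches the possessed pawn as a BP_PlayerCharacter_Sven, and shows the cursor only if that cast succeeds.
; The IA_RightMouseClick action traces under the cursor on the Visibility channel and sends the hit location to SimpleMoveToLocation.
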(event Input|EnhancedActionEvents|EnhancedInputActionIA_RightMouseClick
  (params (ActionValue :type Boolean) (ElapsedSeconds :type Float%20%28double-precision%29) (TriggeredSeconds :type Float%20%28double-precision%29) (InputAction :type Input%20Action%20Object%20Reference :default "/Game/Input/Inputs/IA_RightMouseClick.IA_RightMouseClick"))
  (AI|Navigation|SimpleMovetoLocation self (.Location (Collision|BreakHitResult (.HitResult (Game|Player|GetHitResultUnderCursorbyChannel "TraceTypeQuery1" true))))))

(event EventBeginPlay
  ;[0.01315 0.15 0.1185 0.5] Add Mapping Context
  (Input|AddMappingContext (PlayerController|LocalPlayerSubsystems|GetEnhancedInputLocalPlayerSubsystem) "/Game/Input/IMC_Sven.IMC_Sven" 0 "(bIgnoreAllPressedKeysUntilRelease=True,bForceImmediately=False,bNotifyUserSettings=False)")
  ;[0.01315 0.15 0.1185 0.5] Get Controlled Pawn and Cast to Player Character
  (bind _asbp_player_character_sven (Utilities|Casting|CastToBP_PlayerCharacter_Sven (Pawn|GetControlledPawn)))
  (Variables|Default|SetControlledCharacter _asbp_player_character_sven)
  (Variables|Default|SetbShowMouseCursor true))

(fn ConstructionScript)