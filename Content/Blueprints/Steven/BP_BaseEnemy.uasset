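; BP_BaseEnemy is a base enemy pawn that walks to a target location shortly after it spawns.
; On BeginPlay it waits briefly, confirms its controller is a BP_EnemyAiController, then runs AI MoveTo toward the TargetLocation actor's position.
; Debug prints trace each stage, though the success/failure branch after the move has a constant true condition, so it always reports success.
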(event EventBeginPlay
  (Development|PrintString "\"Enemy spawned\"")
  (Utilities|FlowControl|Delay 2.0)
  (Development|PrintText "starting movement")
  (Utilities|Casting|CastToBP_EnemyAiController (AI|GetAIController self))
  (AI|AIMoveTo self (Transformation|GetActorLocation (Variables|Default|GetTargetLocation)) 0 5e+01 true
    (:then
      (if true
        (Development|PrintString "(\"success\", Color: Green)")
        (else
          (Development|PrintString "failed"))))))

(event Collision|EventActorBeginOverlap
  (params (OtherActor :type Actor%20Object%20Reference)))

(event EventTick
  (params (DeltaSeconds :type Float%20%28single-precision%29)))

(fn ConstructionScript)