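; BP_Bomb is a tower-game projectile that explodes on contact, dealing radial damage around its location.
; A sphere overlap calls Explode, which ignores itself and any BP_BaseTower, then applies damage and destroys the bomb.
; Base and minimum damage are equal, as are inner and outer radii, so damage is uniform across the blast instead of falling off.
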(event OnComponentBeginOverlap(Sphere)
  (params (OverlappedComponent :type Primitive%20Component%20Object%20Reference) (OtherActor :type Actor%20Object%20Reference) (OtherComp :type Primitive%20Component%20Object%20Reference) (OtherBodyIndex :type Integer) (bFromSweep :type Boolean) (SweepResult :type Hit%20Result%20Structure%20%28by%20ref%29))
  (CallFunction|Explode OtherActor))

(event EventBeginPlay)

(event Collision|EventActorBeginOverlap
  (params (OtherActor :type Actor%20Object%20Reference)))

(event EventTick
  (params (DeltaSeconds :type Float%20%28single-precision%29)))

(fn ConstructionScript)

(fn Explode
  (params (HitActor :type Actor%20Object%20Reference))
  (bind _damage (Variables|Default|GetDamage))
  (bind _radius (Variables|Default|GetRadius))
  (if (== HitActor self)
    (return)
    (elif (CallFunction|IsIgnoredClass HitActor)
      (return)
      (else
        (Class|GameplayStatics|ApplyRadialDamagewithFalloff _damage _damage (Transformation|GetActorLocation) _radius _radius 0.0 0 0 self 0 "ECC_Visibility")
        (CallFunction|Destroy)))))

(fn IsIgnoredClass
  (params (Actor :type Actor%20Object%20Reference))
  (Utilities|Casting|CastToBP_BaseTower Actor
    (:then
      (return true))
    (:CastFailed
      (return false))))

(fn Destroy
  (Actor|DestroyActor))

(fn GetProjectileMovement
  (return (Variables|Default|GetProjectileMovement)))