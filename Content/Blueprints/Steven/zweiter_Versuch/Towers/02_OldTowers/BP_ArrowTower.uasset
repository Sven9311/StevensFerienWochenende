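; Arrow tower that fires arrow projectiles at enemies within its range.
; Attack spawns the configured projectile class slightly above the tower, casts it to BP_Arrow, then passes it the first in-range enemy as target and the attack damage.
; It returns false when no enemy is in range.
; The event graph holds only disabled default events, so nothing in this file triggers attacks or fills the enemy list.
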(event EventBeginPlay
  (|CallParentFunction) ; This node is disabled and will not be called.\nDrag off pins to build functionality.
)

(event Collision|EventActorBeginOverlap
  (params (OtherActor :type Actor%20Object%20Reference))
  (|CallParentFunction OtherActor) ; This node is disabled and will not be called.\nDrag off pins to build functionality.
)

(event EventTick
  (params (DeltaSeconds :type Float%20%28single-precision%29))
  (|CallParentFunction DeltaSeconds) ; This node is disabled and will not be called.\nDrag off pins to build functionality.
)

(fn ConstructionScript
  (|CallParentFunction))

(fn Attack
  (if (> (Utilities|Array|Length (Variables|Default|GetEnemiesInRange)) 0)
    (bind _returnvalue (Game|SpawnActorfromClass (Variables|Default|GetProjectileClass) (CallFunction|GetArrowSpawnTransform) "Undefined" "MultiplyWithRoot" 0 0))
    (bind _asbp_arrow (Utilities|Casting|CastToBP_Arrow _returnvalue))
    (Default|SetTarget _asbp_arrow (Utilities|Array|Get(acopy) (Variables|Default|GetEnemiesInRange)))
    (Default|SetDamage _asbp_arrow (Variables|Default|GetAttackDamage))
    (return true)
    (else
      (return false))))

(fn GetArrowSpawnTransform
  (bind _returnvalue (Transformation|GetActorTransform))
  (return (Math|Transform|MakeTransform (Math|Vector|MakeVector (.x (.location _returnvalue)) (.y (.location _returnvalue)) (+ (.z (.location _returnvalue)) 1e+02)) (.rotation _returnvalue) (.scale _returnvalue))))