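; BP_BlowFlowerProjectile is a straight-flying projectile that destroys enemies it hits.
; On BeginPlay it stores the direction to TargetLocation, then moves along it each Tick at ProjectileSpeed with a swept offset, without homing.
; When its static mesh hits a BP_BaseEnemy, it calls OnTargetDestroyed with that enemy and destroys it.
; The projectile destroys itself on any hit.
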(event OnComponentHit(StaticMesh)
  (params (HitComponent :type Primitive%20Component%20Object%20Reference) (OtherActor :type Actor%20Object%20Reference) (OtherComp :type Primitive%20Component%20Object%20Reference) (NormalImpulse :type Vector :default "0, 0, 0") (Hit :type Hit%20Result%20Structure%20%28by%20ref%29))
  (bind _asbp_base_enemy (Utilities|Casting|CastToBP_BaseEnemy OtherActor)
    (:then
      (Default|CallOnTargetDestroyed _asbp_base_enemy)
      (Actor|DestroyActor _asbp_base_enemy))
    (:CastFailed
      _))
  (Actor|DestroyActor))

(event EventBeginPlay
  (|CallParentFunction)
  (Variables|Default|SetTargetDirection (- (Variables|Default|GetTargetLocation) (Transformation|GetActorLocation))))

(event Collision|EventActorBeginOverlap
  (params (OtherActor :type Actor%20Object%20Reference))
  (|CallParentFunction OtherActor) ; This node is disabled and will not be called.\nDrag off pins to build functionality.
)

(event EventTick
  (params (DeltaSeconds :type Float%20%28single-precision%29))
  (|CallParentFunction DeltaSeconds)
  (Transformation|AddActorWorldOffset (* (* (Math|Vector|Normalize (Variables|Default|GetTargetDirection)) (Variables|Default|GetProjectileSpeed)) (Utilities|Time|GetWorldDeltaSeconds)) true))

(fn ConstructionScript
  (|CallParentFunction))