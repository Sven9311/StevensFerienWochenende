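; Bomb tower that lobs an explosive projectile at the first enemy in its range.
; Attack spawns the projectile 100 units above the tower, passes it damage and blast radius, and reports whether any enemy was available.
; The arc uses a fixed upward speed and scales horizontal velocity by target offset over a constant flight time, with no target leading.
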(event EventBeginPlay
  (|CallParentFunction) ; This node is disabled and will not be called.\nDrag off pins to build functionality.
)

(event Collision|EventActorBeginOverlap
  (params (OtherActor :type Actor%20Object%20Reference))
  (|CallParentFunction OtherActor) ; This node is disabled and will not be called.\nDrag off pins to build functionality.
)

(event EventTick
  (params (DeltaSeconds :type Float%20%28single-precision%29))
  (|CallParentFunction DeltaSeconds) ; This node is disabled and will not be called.\nDrag off pins to build functionality.
)

(fn ConstructionScript
  (|CallParentFunction))

(fn Attack
  (if (> (Utilities|Array|Length (Variables|Default|GetEnemiesInRange)) 0)
    (bind _returnvalue (Game|SpawnActorfromClass (Variables|Default|GetProjectileClass) (CallFunction|GetBombSpawnTransform) "AlwaysSpawn" "MultiplyWithRoot" 0 0))
    (bind _asbp_bomb (Utilities|Casting|CastToBP_Bomb _returnvalue))
    (Variables|/Game/Blueprints/Steven/zweiter_Versuch/Towers/Projectiles/BP_Bomb.BP_Bomb_C|SetDamage _asbp_bomb (Variables|Default|GetAttackDamage))
    (Variables|/Game/Blueprints/Steven/zweiter_Versuch/Towers/Projectiles/BP_Bomb.BP_Bomb_C|SetRadius _asbp_bomb (Variables|Default|GetBombRadius))
    (Variables|/Script/Engine.MovementComponent|SetVelocity (Default|GetProjectileMovement _asbp_bomb) (Math|Vector|MakeVector (.x (/ (- (Transformation|GetActorLocation (Utilities|Array|Get(acopy) (Variables|Default|GetEnemiesInRange))) (Transformation|GetActorLocation _asbp_bomb)) 1.0475)) (.y (/ (- (Transformation|GetActorLocation (Utilities|Array|Get(acopy) (Variables|Default|GetEnemiesInRange))) (Transformation|GetActorLocation _asbp_bomb)) 1.0475)) 4.9e+02))
    (return true)
    (else
      (return false))))

(fn GetBombSpawnTransform
  (bind _returnvalue (Transformation|GetActorTransform))
  (return (Math|Transform|MakeTransform (Math|Vector|MakeVector (.x (.location _returnvalue)) (.y (.location _returnvalue)) (+ (.z (.location _returnvalue)) 1e+02)) (.rotation _returnvalue) (.scale _returnvalue))))