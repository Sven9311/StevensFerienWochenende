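; BP_DynamicPanel is a grid panel that wears from grass to dirt as it is stepped on, forming a trampled path.
; On BeginPlay it gives its cube a dynamic material instance with a GrassOrDirt scalar.
; Each box overlap raises that scalar one step and stops the regrowth timer; leaving starts a looping timer that lowers it step by step.
; A debug counter tracks both; older threshold and timeline logic is unconnected.
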(event OnComponentBeginOverlap(Box)
  (params (OverlappedComponent :type Primitive%20Component%20Object%20Reference) (OtherActor :type Actor%20Object%20Reference) (OtherComp :type Primitive%20Component%20Object%20Reference) (OtherBodyIndex :type Integer) (bFromSweep :type Boolean) (SweepResult :type Hit%20Result%20Structure%20%28by%20ref%29))
  (Utilities|Time|ClearandInvalidateTimerbyHandle (stale OnComponentEndOverlap(Box) _returnvalue))
  (CallFunction|TrampelpfadBilden))

(event OnComponentEndOverlap(Box)
  (params (OverlappedComponent :type Primitive%20Component%20Object%20Reference) (OtherActor :type Actor%20Object%20Reference) (OtherComp :type Primitive%20Component%20Object%20Reference) (OtherBodyIndex :type Integer))
  (bind _returnvalue (Utilities|Time|SetTimerbyEvent (delegate Custom|gras%20über%20die%20sache%20wachsen%20lassen) 5.0 true)))

(event Custom|gras%20über%20die%20sache%20wachsen%20lassen
  (bind _returnvalue (Rendering|Material|GetScalarParameterValue (Variables|Default|GetDynamicMaterialInstance) "GrassOrDirt" :!class /Script/Engine.MaterialInstanceDynamic))
  (if (> _returnvalue 0.0)
    (bind _result (Math|Integer|DecrementInt (Variables|Default|GetZählerBetreten))
      (:%20%20
        (Development|PrintString (Utilities|String|Append "Nachgewachsen:  " (Utilities|String|ToString(Integer) _result)) true true "(R=0.000000,G=0.660000,B=1.000000,A=1.000000)" 2.0 "")
        (Rendering|Material|SetScalarParameterValue (Variables|Default|GetDynamicMaterialInstance) "GrassOrDirt" (- _returnvalue 0.25) :!class /Script/Engine.MaterialInstanceDynamic)))))

(event Custom|Trampelpfad%20bilden
  (bind _dynamicmaterialinstance (Variables|Default|GetDynamicMaterialInstance))
  (bind _returnvalue (Rendering|Material|GetScalarParameterValue _dynamicmaterialinstance "GrassOrDirt" :!class /Script/Engine.MaterialInstanceDynamic))
  (Development|PrintString (Utilities|String|ToString(Float) _returnvalue) true true "(R=0.000000,G=0.660000,B=1.000000,A=1.000000)" 0.0)
  (if (< _returnvalue 1.0)
    (Rendering|Material|SetScalarParameterValue _dynamicmaterialinstance "GrassOrDirt" (+ _returnvalue 0.25) :!class /Script/Engine.MaterialInstanceDynamic)
    (bind _result (Math|Integer|IncrementInt (Variables|Default|GetZählerBetreten))
      (:%20%20
        (Development|PrintString (Utilities|String|Append "Betreten:  " (Utilities|String|ToString(Integer) _result)) true true "(R=0.000000,G=0.660000,B=1.000000,A=1.000000)" 2.0 "")))))

(event EventBeginPlay
  ;[0.15 0.15 0.15 0.5] Create Material
  (bind _returnvalue (Rendering|Material|CreateDynamicMaterialInstance (Rendering|Material|GetMaterial (Variables|Default|GetCube) 0) "" "None" :!class /Script/Engine.KismetMaterialLibrary))
  (bind _output_get (Variables|Default|SetDynamicMaterialInstance _returnvalue))
  (Rendering|Material|SetMaterial (Variables|Default|GetCube) 0 _output_get))

(fn ConstructionScript)

(fn NotWalkedOver
  (return true))