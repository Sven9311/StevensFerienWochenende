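; BP_Enemy is an enemy actor that takes damage and pays money to the player when it dies.
; On BeginPlay it binds to OnTakeAnyDamage, which calls TakeDamage; this sets HP to Damage minus HP (operands reversed from a usual subtraction) and calls Die at zero or below.
; Die sends MoneyDrop to player 0's BP_PlayerController via ReceiveMoney if the cast succeeds, then destroys the actor either way.
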(event Custom|OnTakeAnyDamage_Event
  (params (DamagedActor :type Actor%20Object%20Reference) (Damage :type Float%20%28single-precision%29) (DamageType :type Damage%20Type%20Object%20Reference) (InstigatedBy :type Controller%20Object%20Reference) (DamageCauser :type Actor%20Object%20Reference))
  (CallFunction|TakeDamage Damage))

(event EventBeginPlay
  (EventDispatchers|AssignOnTakeAnyDamage (delegate Custom|OnTakeAnyDamage_Event)))

(event Collision|EventActorBeginOverlap
  (params (OtherActor :type Actor%20Object%20Reference)))

(event EventTick
  (params (DeltaSeconds :type Float%20%28single-precision%29)))

(fn ConstructionScript)

(fn TakeDamage
  (params (Damage :type Float%20%28double-precision%29))
  (bind _output_get (Variables|Default|SetHP (- Damage (Variables|Default|GetHP))))
  (if (<= _output_get 0.0)
    (CallFunction|Die)))

(fn Die
  (bind _asbp_player_controller (Utilities|Casting|CastToBP_PlayerController (Game|GetPlayerController 0))
    (:then
      (Default|ReceiveMoney _asbp_player_controller (Variables|Default|GetMoneyDrop))
      (Actor|DestroyActor))
    (:CastFailed
      (Actor|DestroyActor))))