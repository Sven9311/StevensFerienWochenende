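; Blow flower tower that automatically fires homing projectiles at the closest enemy in range.
; Each tick off cooldown, it picks the nearest entry in EnemiesInRange and spawns a BP_BlowFlowerProjectile homing on a scene component newly added to that target.
; A continuously running AttackSpeed timer clears the cooldown, and each projectile's OnTargetDestroyed event removes the destroyed target from the list.
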(event Custom|OnTargetDestroyed_Event
  (params (DestroyTarget :type Actor%20Object%20Reference))
  (Utilities|Array|RemoveItem (Variables|Default|GetEnemiesInRange) DestroyTarget))

(event EventTick
  (params (DeltaSeconds :type Float%20%28single-precision%29))
  (|CallParentFunction 0.0)
  (if (Variables|Default|GetIsOnCooldown)
    _
    (else
      (CallFunction|FindClosestEnemyinRange)
      (Development|PrintString (Utilities|GetDisplayName (Variables|Default|GetClosestTarget)) true true "(R=0.000000,G=0.660000,B=1.000000,A=1.000000)" 2.0 "1")
      (Variables|Default|GetClosestTarget
        (:then
          (bind _returnvalue (Game|SpawnActorfromClass "/Game/Blueprints/Steven/BP_BlowFlowerProjectile.BP_BlowFlowerProjectile_C" (Transformation|GetWorldTransform (Variables|Default|GetProjectileSpawn)) "Undefined" "MultiplyWithRoot" 0 (Transformation|GetActorLocation (Variables|Default|GetClosestTarget)) 0))
          (bind _returnvalue_2 (AddComponent|AddSceneComponent (Variables|Default|GetClosestTarget) false))
          (Variables|/Script/Engine.ProjectileMovementComponent|SetHomingTargetComponent (Variables|/Game/Blueprints/Steven/BP_BaseProjectile.BP_BaseProjectile_C|GetProjectileMovement _returnvalue) _returnvalue_2)
          (EventDispatchers|AssignOnTargetDestroyed _returnvalue (delegate Custom|OnTargetDestroyed_Event))
          (Variables|Default|SetIsOnCooldown true))
        (:else
          _))))
  (Variables|Default|SetCurrentTime (+ (Variables|Default|GetCurrentTime) (Utilities|Time|GetWorldDeltaSeconds)))
  (if (>= (Variables|Default|GetCurrentTime) (Variables|Default|GetAttackSpeed))
    (Variables|Default|SetIsOnCooldown false)
    (Variables|Default|SetCurrentTime 0.0)))

(event EventBeginPlay
  (Variables|Default|SetClosestTargetRange (Variables|Default|GetAttackRange))
  (CallFunction|FindClosestEnemyinRange))

(fn ConstructionScript
  (|CallParentFunction))

(fn FindClosestEnemyinRange
  (for _array_element (Variables|Default|GetEnemiesInRange)
    (if (< (Transformation|GetDistanceTo self _array_element) (Variables|Default|GetClosestTargetRange))
      (Variables|Default|SetClosestTargetRange (Transformation|GetDistanceTo self _array_element))
      (Variables|Default|SetClosestTarget _array_element)))
  (Variables|Default|SetClosestTargetRange (Variables|Default|GetAttackRange)))