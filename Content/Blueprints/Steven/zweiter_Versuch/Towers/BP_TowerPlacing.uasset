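; BP_TowerPlacing is a placement block that holds a single tower in what appears to be a tower-defense game.
; SpawnTower spawns the given class at TowerLocation only when the block is empty, then links tower and block to each other.
; DestroyTower removes a valid tower, and HasTower reports occupancy.
; CreateMaterial gives the cube a dynamic stone material with randomized XCord/YCord parameters, though nothing in this Blueprint calls it.
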(event EventBeginPlay)

(event Collision|EventActorBeginOverlap
  (params (OtherActor :type Actor%20Object%20Reference)))

(event EventTick
  (params (DeltaSeconds :type Float%20%28single-precision%29)))

(fn ConstructionScript)

(fn CreateMaterial
  (bind _returnvalue (Rendering|Material|CreateDynamicMaterialInstance (Variables|Default|GetCube) 0 "/Game/Blueprints/Steven/zweiter_Versuch/Assets/Materials/MI_Stone.MI_Stone" "None" :!class /Script/Engine.PrimitiveComponent))
  (bind _output_get (Variables|Default|SetMaterialInstance _returnvalue))
  (Rendering|Material|SetScalarParameterValue _output_get "XCord" (Math|Conversions|ToFloat(Integer) (Math|Random|RandomIntegerinRange 0 1)) :!class /Script/Engine.MaterialInstanceDynamic)
  (Rendering|Material|SetScalarParameterValue _output_get "YCord" (Math|Conversions|ToFloat(Integer) (Math|Random|RandomIntegerinRange 0 1)) :!class /Script/Engine.MaterialInstanceDynamic))

(fn HasTower
  (return (Utilities|IsValid (Variables|Default|GetTower))))

(fn SpawnTower
  (params (TowerClass :type BP%20Base%20Tower%20Class%20Reference))
  (if (CallFunction|HasTower)
    (return)
    (else
      (bind _returnvalue (Game|SpawnActorfromClass TowerClass (Math|Transform|MakeTransform (Transformation|GetWorldLocation (Variables|Default|GetTowerLocation)) "0, 0, 0" "1.000000,1.000000,1.000000") "AlwaysSpawn" "MultiplyWithRoot" 0 0))
      (bind _output_get (Variables|Default|SetTower _returnvalue))
      (Variables|/Game/Blueprints/Steven/zweiter_Versuch/Towers/BP_BaseTower.BP_BaseTower_C|SetTowerPlacingBlock _output_get self))))

(fn DestroyTower
  (bind _tower (Variables|Default|GetTower))
  (if (Utilities|IsValid _tower)
    (Actor|DestroyActor _tower)))