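; BP_EnemySpawner is a spawner actor that releases a limited number of BP_BaseEnemy2 enemies over time at its own location.
; On BeginPlay it starts a looping timer that spawns one enemy per interval until the configured count is reached.
; Each spawned enemy receives the spawner's TargetPoint as its GoalPoint.
; The timer is never cleared, so it keeps printing a completion debug message afterwards.
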(event Custom|SpawnEnemy
  (if (< (Variables|Default|GetSpawnedCount%20%28intern%29) (Variables|Default|GetNumberOfEnemies))
    (bind _returnvalue (Game|SpawnActorfromClass "/Game/Blueprints/Steven/Neuer_Versuch/BP_BaseEnemy2.BP_BaseEnemy2_C" (Math|Transform|MakeTransform (Transformation|GetActorLocation)) "AdjustIfPossibleButAlwaysSpawn" "MultiplyWithRoot" 0 0))
    (bind _asbp_base_enemy_2 (Utilities|Casting|CastToBP_BaseEnemy2 _returnvalue)
      (:then
        (Variables|/Game/Blueprints/Steven/Neuer_Versuch/BP_BaseEnemy2.BP_BaseEnemy2_C|SetGoalPoint _asbp_base_enemy_2 (Variables|Default|GetTargetPoint))
        (Math|Integer|IncrementInt (Variables|Default|GetSpawnedCount%20%28intern%29)))
      (:CastFailed
        (Development|PrintString "FAILED TO CAST !!!!!_____" true true "(R=1.000000,G=0.041245,B=0.000000,A=1.000000)")))
    (else
      (Development|PrintString "Alle Gegner gespawned!" true true "(R=1.000000,G=0.079628,B=0.000000,A=1.000000)"))))

(event EventBeginPlay
  (Variables|Default|SetSpawnedCount%20%28intern%29 0)
  (Utilities|Time|SetTimerbyEvent (delegate Custom|SpawnEnemy) (Variables|Default|GetSpawnInterval) true))

(fn ConstructionScript)