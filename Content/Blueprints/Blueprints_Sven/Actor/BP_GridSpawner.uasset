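; BP_GridSpawner is an actor that fills a rectangular grid with spawned tile actors when play begins.
; Nested loops over GridSizeY and GridSizeX spawn one GridTiles actor per cell at a fixed 200-unit spacing, at the spawner's height.
; Indices start at one, so the first tile sits one spacing away from the spawner's location in both X and Y.
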(event EventBeginPlay
  (bind _returnvalue (Transformation|GetActorLocation))
  (for _index (range 1 (Variables|Default|GetGridSizeY))
    (Variables|Default|SetCurrentYIndex _index)
    (for _index_2 (range 1 (Variables|Default|GetGridSizeX))
      (bind _output_get (Variables|Default|SetCurrentXIndex _index_2))
      (Game|SpawnActorfromClass (Variables|Default|GetGridTiles) (Math|Transform|MakeTransform (Math|Vector|MakeVector (+ (* _output_get 200) (.x _returnvalue)) (+ (.y _returnvalue) (* (Variables|Default|GetCurrentYIndex) 200)) (.z _returnvalue)) "0, 0, 0" "1.000000,1.000000,1.000000") "Undefined" "MultiplyWithRoot" 0 0))))

(fn ConstructionScript)