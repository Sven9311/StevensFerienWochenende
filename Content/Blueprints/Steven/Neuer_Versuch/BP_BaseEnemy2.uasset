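; BP_BaseEnemy2 is an enemy base Blueprint that walks toward a GoalPoint actor.
; Shortly after BeginPlay it checks that GoalPoint is valid and runs AI MoveTo to that actor's location.
; StartMoving ignores its Target input and clears GoalPoint, so its SimpleMoveToLocation, aimed at the enemy's own location, never runs.
; The destruction events are empty stubs.
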(event Custom|OnEnemyDestroyed_Event)

(event EventBeginPlay
  (Utilities|FlowControl|Delay 0.2)
  (if (Utilities|IsValid (Variables|Default|GetGoalPoint))
    (AI|AIMoveTo self (Transformation|GetActorLocation (Variables|Default|GetGoalPoint)) 0 1e+02 false)))

(event Collision|EventActorBeginOverlap
  (params (OtherActor :type Actor%20Object%20Reference)))

(event EventTick
  (params (DeltaSeconds :type Float%20%28single-precision%29)))

(event EventDestroyed)

(fn ConstructionScript)

(fn StartMoving
  (params (Target :type Actor%20Object%20Reference))
  (Variables|Default|SetGoalPoint 0)
  (if (Utilities|IsValid (Variables|Default|GetGoalPoint))
    (AI|Navigation|SimpleMovetoLocation (AI|GetAIController self) (Transformation|GetActorLocation))))