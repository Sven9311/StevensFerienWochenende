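; BP_DefineNextPoint is a behavior tree task that gives an enemy its next path point to move to.
; It casts the owner to BP_EnemyController and reads the actor at MoveIndex in the Path array of that controller's Spawner.
; It writes that actor's location to the Location blackboard key, increments MoveIndex and finishes successfully.
; The index has no bounds check or wrap, and a failed cast never finishes the task.
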(event EventReceiveExecute
  (params (OwnerActor :type Actor%20Object%20Reference))
  (bind _asbp_enemy_controller (Utilities|Casting|CastToBP_EnemyController OwnerActor))
  (AI|BehaviorTree|SetBlackboardValueasVector (Variables|Default|GetLocation) (Transformation|GetActorLocation (Utilities|Array|Get(acopy) (Variables|/Game/Blueprints/Steven/zweiter_Versuch/BP_EnemySpawner.BP_EnemySpawner_C|GetPath (Variables|/Game/Blueprints/Steven/zweiter_Versuch/BP_EnemyController.BP_EnemyController_C|GetSpawner _asbp_enemy_controller)) (Variables|/Game/Blueprints/Steven/zweiter_Versuch/BP_EnemyController.BP_EnemyController_C|GetMoveIndex _asbp_enemy_controller))))
  (Math|Integer|IncrementInt (Variables|/Game/Blueprints/Steven/zweiter_Versuch/BP_EnemyController.BP_EnemyController_C|GetMoveIndex _asbp_enemy_controller)
    (:%20%20
      (AI|BehaviorTree|FinishExecute true))))