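; Player controller for a tower defense game that handles mouse clicks, tower UI and the player's money.
; On BeginPlay it adds the input mapping, shows the cursor and creates hidden placement and upgrade widgets.
; IA_Click traces under the cursor, opening the placement UI for placing blocks or the upgrade UI with a clicked tower's options.
; Functions add or conditionally spend money, while Tick prints the hovered grid cell as debug.
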(event Input|EnhancedActionEvents|EnhancedInputActionIA_Click
  (params (ActionValue :type Boolean) (ElapsedSeconds :type Float%20%28double-precision%29) (TriggeredSeconds :type Float%20%28double-precision%29) (InputAction :type Input%20Action%20Object%20Reference :default "/Game/Blueprints/Steven/zweiter_Versuch/Player/Input/IA_Click.IA_Click"))
  (bind _hitresult (Game|Player|GetHitResultUnderCursorbyChannel "TraceTypeQuery1" true))
  (bind _asbp_tower_placing (Utilities|Casting|CastToBP_TowerPlacing (.hitactor _hitresult))
    (:then
      (CallFunction|ShowAddTowerUI _asbp_tower_placing))
    (:CastFailed
      (bind _asbp_base_tower (Utilities|Casting|CastToBP_BaseTower (.hitactor _hitresult)))
      (CallFunction|ShowUpgradeTowerUI _asbp_base_tower))))

(event EventBeginPlay
  (Development|PrintString "Hello")
  (Input|AddMappingContext (PlayerController|LocalPlayerSubsystems|GetEnhancedInputLocalPlayerSubsystem) "/Game/Blueprints/Steven/zweiter_Versuch/Player/Input/IMC_Default.IMC_Default" 0 "(bIgnoreAllPressedKeysUntilRelease=True,bForceImmediately=False,bNotifyUserSettings=False)")
  (Variables|Default|SetbShowMouseCursor true)
  (bind _returnvalue (UserInterface|CreateWidget "/Game/Blueprints/Steven/zweiter_Versuch/UI/BP_TowerPlacingUi.BP_TowerPlacingUi_C"))
  (bind _output_get (Variables|Default|SetAddTowerUI _returnvalue))
  (UserInterface|Viewport|AddtoViewport _output_get 0)
  (Widget|SetVisibility _output_get "Hidden")
  (bind _returnvalue_2 (UserInterface|CreateWidget "/Game/Blueprints/Steven/zweiter_Versuch/UI/BP_TowerUpgradeUI.BP_TowerUpgradeUI_C"))
  (bind _output_get_2 (Variables|Default|SetUpgradeTowerUI _returnvalue_2))
  (UserInterface|Viewport|AddtoViewport _output_get_2 0)
  (Widget|SetVisibility _output_get_2 "Hidden"))

(event EventTick
  (params (DeltaSeconds :type Float%20%28single-precision%29))
  (bind (_hit _location) (CallFunction|GetLocationUnderCursor))
  (if _hit
    (Development|PrintString (Utilities|String|ToString(Vector) (Default|GetGridLocation (Variables|Default|GetBP_Grid) _location)) true true "(R=0.000000,G=0.660000,B=1.000000,A=1.000000)" 0.0)))

(fn ConstructionScript)

(fn ReceiveMoney
  (params (Amount :type Integer))
  (Variables|Default|SetMoney (+ Amount (Variables|Default|GetMoney))))

(fn HideAddTowerUi
  (Widget|SetVisibility (Variables|Default|GetAddTowerUI) "Hidden"))

(fn SpendMoney
  (params (Amount :type Integer))
  (if (>= (Variables|Default|GetMoney) Amount)
    (Variables|Default|SetMoney (- (Variables|Default|GetMoney) Amount))
    (return true)
    (else
      (return false))))

(fn ShowAddTowerUI
  (params (TowerPlacingBlock :type BP%20Tower%20Placing%20Object%20Reference))
  (bind _addtowerui (Variables|Default|GetAddTowerUI))
  (Variables|/Game/Blueprints/Steven/zweiter_Versuch/UI/BP_TowerPlacingUi.BP_TowerPlacingUi_C|SetPlacingTowerBlock _addtowerui TowerPlacingBlock)
  (Widget|SetVisibility _addtowerui "Visible"))

(fn ShowUpgradeTowerUI
  (params (ClickedTower :type BP%20Base%20Tower%20Object%20Reference))
  (bind _upgradetowerui (Variables|Default|GetUpgradeTowerUI))
  (Widget|SetVisibility _upgradetowerui "Visible")
  (Default|SetOptions _upgradetowerui (Variables|/Game/Blueprints/Steven/zweiter_Versuch/Towers/BP_BaseTower.BP_BaseTower_C|GetTowerPlacingBlock ClickedTower) (Default|GetPossibleUpgrades ClickedTower)))

(fn GetLocationUnderCursor
  (bind _returnvalue (Game|GetPlayerController 0))
  (bind _hitresult (Game|Player|GetHitResultUnderCursorbyChannel _returnvalue "TraceTypeQuery1" true))
  (return (.bblockinghit _hitresult) (.location _hitresult)))